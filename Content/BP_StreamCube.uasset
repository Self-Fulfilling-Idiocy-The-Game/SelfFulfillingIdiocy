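; BP_StreamCube is an interactable actor that swaps streamed levels when the player presses E while looking at it.
; On BeginPlay it enables player input and loads the House sublevel without blocking.
; OnLookat and OnLookAway events toggle a Looking flag that gates the key press.
; The swap unloads House and loads FTL once; the StreamedLevel state has no branch back to House.
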(event EventBeginPlay
  (Input|EnableInput (Game|GetPlayerController 0))
  (Game|LoadStreamLevel(byName) "House" true)
  (Variables|Default|SetStreamedLevel 1))

(event Collision|EventActorBeginOverlap
  (params (OtherActor :type Actor%20Object%20Reference)))

(event EventOnLookAway
  (Variables|Default|SetLooking false))

(event EventOnLookat
  (Variables|Default|SetLooking true))

(event EventTick
  (params (DeltaSeconds :type Float%20%28single-precision%29)))

(event Input|KeyboardEvents|E
  (params (Key :type Key%20Structure))
  (:Pressed
    (if (Variables|Default|GetLooking)
      (if (== (Variables|Default|GetStreamedLevel) 1)
        (Game|UnloadStreamLevel(byName) "House")
        (Game|LoadStreamLevel(byName) "FTL" true)
        (Variables|Default|SetStreamedLevel 2)))))

(fn ConstructionScript)